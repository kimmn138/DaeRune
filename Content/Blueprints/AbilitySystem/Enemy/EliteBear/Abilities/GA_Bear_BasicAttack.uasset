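; Gameplay ability for the Elite Bear enemy's basic melee attack.
; On activation it turns the bear to face its combat target, notifies the enemy base, and plays a tagged attack montage.
; At the montage's gameplay event, it sphere-checks around the attack socket, damages live non-friendly actors and triggers their blood effects.
; Any hit fires a melee impact gameplay cue before the ability ends, without stopping the montage.
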(event `self.K2_ActivateAbility`
  (bind _returnvalue (`self.GetAvatarActorFromActorInfo`))
  (bind _returnvalue_2 (`self.GetAvatarActorFromActorInfo`))
  (bind (_montage _montagetag _sockettag) (break `TaggedMontage` (`self.TaggedMontage`)))
  (set `self.HasHitTarget` false)
  (bind _returnvalue_3 (message `EnemyInterface.GetCombatTarget` _returnvalue))
  (bind _ascombat_interface (cast `CombatInterface` _returnvalue))
  (`CombatInterface.UpdateFacingTarget` _ascombat_interface (`Actor.K2_GetActorLocation` _returnvalue_3))
  (bind _asbp_enemy_base (cast `/Game/Blueprints/Character/BP_EnemyBase` _returnvalue))
  (`DREnemy.OnAttackExecuted` _asbp_enemy_base)
  (`AbilityTask_PlayMontageAndWait.CreatePlayMontageAndWaitProxy` "None" _montage 1.0 "None" false
    (:`then`
      (`AbilityTask_WaitGameplayEvent.WaitGameplayEvent` _montagetag null
        (:`EventReceived`
          (bind _returnvalue_4 (message `CombatInterface.GetCombatSocketLocation` _returnvalue_2 _sockettag))
          (set `self.CombatSocketLocation` _returnvalue_4)
          (bind _outoverlappingactors (`DRAbilitySystemLibrary.GetLiveObjectsWithinRadius` _returnvalue_2 (`|MakeArray` _returnvalue_2) 100.0 (`self.CombatSocketLocation`)))
          (for _array_element _outoverlappingactors
            (if (`DRAbilitySystemLibrary.IsNotFriend` (`self.GetAvatarActorFromActorInfo`) _array_element)
              (`DRAbilitySystemLibrary.ApplyDamageEffect` (`self.MakeDamageEffectParamsFromClassDefaults` _array_element))
              (set `self.HasHitTarget` true)
              (message `CombatInterface.GetBloodEffect` _array_element)))
          (if (`self.HasHitTarget`)
            (bind _returnvalue_5 (message `EnemyInterface.GetCombatTarget` (`self.GetAvatarActorFromActorInfo`)))
            (`self.K2_ExecuteGameplayCueWithParams` (struct :`TagName` "GameplayCue.MeleeImpact") (`AbilitySystemBlueprintLibrary.MakeGameplayCueParameters` 0.0 0.0 (struct) (struct) (struct) (`BlueprintGameplayTagLibrary.MakeGameplayTagContainerFromTag` (`.MontageTag` (break `TaggedMontage` (`self.TaggedMontage`)))) (struct) (`self.CombatSocketLocation`) (0.0 0.0 0.0) null null _returnvalue_5)))
          (`self.K2_EndAbility`))))
    (:`OnCompleted`
      (`self.K2_EndAbility` :!label _label))
    (:`OnInterrupted`
      (goto _label))
    (:`OnCancelled`
      (goto _label))))