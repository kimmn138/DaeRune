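; GA_DeathExplosion is an enemy gameplay ability that detonates its avatar, damaging live objects around it and then destroying the avatar.
; On activation it fires the enemy explosion gameplay cue and draws a brief debug sphere matching the blast radius.
; A radius query that excludes the avatar supplies targets, each receiving damage built from class defaults and setting HasHitTarget.
; The ability ends immediately after destroying the avatar.
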(event `self.K2_ActivateAbility`
  (bind _returnvalue (`self.GetAvatarActorFromActorInfo`))
  (bind _returnvalue_2 (`Actor.K2_GetActorLocation` _returnvalue))
  (set `self.HasHitTarget` false)
  (`KismetSystemLibrary.DrawDebugSphere` _returnvalue_2 400.0 12 (struct :`R` 0.06597 :`B` 1.0 :`A` 1.0) 1.0)
  (`self.K2_ExecuteGameplayCue` (struct :`TagName` "GameplayCue.Enemy.Explosion"))
  (bind _outoverlappingactors (`DRAbilitySystemLibrary.GetLiveObjectsWithinRadius` _returnvalue (`|MakeArray` _returnvalue) 400.0 _returnvalue_2))
  (for _array_element _outoverlappingactors
    (`/Engine/EditorBlueprintResources/StandardMacros.IsValid` _array_element
      (:`Is Valid`
        (`DRAbilitySystemLibrary.ApplyDamageEffect` (`self.MakeDamageEffectParamsFromClassDefaults` _array_element))
        (set `self.HasHitTarget` true))))
  (`Actor.K2_DestroyActor` (`self.GetAvatarActorFromActorInfo`))
  (`self.K2_EndAbility`))