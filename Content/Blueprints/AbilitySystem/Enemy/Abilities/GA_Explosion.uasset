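; Enemy self-destruct ability that damages live actors around the avatar in a radial explosion, then destroys the avatar.
; A random tagged attack montage plays, and its gameplay event triggers an overlap query that applies class-default damage and blood effects to each target.
; Any hit also fires the melee impact gameplay cue, tagged with the montage tag.
; Debug prints and a debug sphere remain in the graph.
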(event `self.K2_ActivateAbility`
  (bind _returnvalue (`self.GetAvatarActorFromActorInfo`))
  (bind _returnvalue_2 (`self.GetAvatarActorFromActorInfo`))
  (bind _returnvalue_3 (`Actor.K2_GetActorLocation` _returnvalue_2))
  (`KismetSystemLibrary.PrintString` "Hello1")
  (set `self.HasHitTarget` false)
  (bind _returnvalue_4 (message `CombatInterface.GetAttackMontages` (`self.GetAvatarActorFromActorInfo`)))
  (bind _output_get (set `self.TaggedMontage` (`self.GetRandomTaggedMontageFromArray` _returnvalue_4)))
  (`KismetSystemLibrary.PrintString` "Hello2")
  (bind (_montage _montagetag) (break `TaggedMontage` _output_get))
  (`AbilityTask_PlayMontageAndWait.CreatePlayMontageAndWaitProxy` "None" _montage 1.0 "None" false
    (:`then`
      (`KismetSystemLibrary.PrintString` "Hello3")
      (`AbilityTask_WaitGameplayEvent.WaitGameplayEvent` _montagetag null
        (:`EventReceived`
          (`KismetSystemLibrary.PrintString` "Hello4")
          (`KismetSystemLibrary.DrawDebugSphere` _returnvalue_3 400.0 12 (struct :`R` 0.06597 :`B` 1.0 :`A` 1.0) 1.0)
          (bind _outoverlappingactors (`DRAbilitySystemLibrary.GetLiveObjectsWithinRadius` _returnvalue_2 (`|MakeArray` _returnvalue_2) 400.0 _returnvalue_3))
          (for _array_element _outoverlappingactors
            (`DRAbilitySystemLibrary.ApplyDamageEffect` (`self.MakeDamageEffectParamsFromClassDefaults` _array_element))
            (set `self.HasHitTarget` true)
            (message `CombatInterface.GetBloodEffect` _array_element))
          (if (`self.HasHitTarget`)
            (bind _returnvalue_5 (message `EnemyInterface.GetCombatTarget` _returnvalue))
            (`self.K2_ExecuteGameplayCueWithParams` (struct :`TagName` "GameplayCue.MeleeImpact") (`AbilitySystemBlueprintLibrary.MakeGameplayCueParameters` 0.0 0.0 (struct) (struct) (struct) (`BlueprintGameplayTagLibrary.MakeGameplayTagContainerFromTag` (`.MontageTag` (break `TaggedMontage` (`self.TaggedMontage`)))) (struct) (0.0 0.0 0.0) (0.0 0.0 0.0) null null _returnvalue_5)))
          (`Actor.K2_DestroyActor` _returnvalue)
          (`self.K2_EndAbility`))))
    (:`OnCompleted`
      (`KismetSystemLibrary.PrintString` "Hello5" :!label _label)
      (`self.K2_EndAbility`))
    (:`OnInterrupted`
      (goto _label))
    (:`OnCancelled`
      (goto _label))))