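; Gameplay ability for the DragonFly flying enemy's basic attack, which fires a projectile at its combat target.
; On activation it notifies the enemy and plays a tagged montage, waiting once for that montage's gameplay event tag.
; The event spawns the projectile from the tagged socket with optional pitch override, then increments the attack count in the AI blackboard.
; The ability ends when the montage completes, is interrupted or is cancelled.
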(event `self.K2_ActivateAbility`
  (bind _returnvalue (`self.GetAvatarActorFromActorInfo`))
  (bind (_montage _montagetag _sockettag) (break `TaggedMontage` (`self.TaggedMontage`)))
  (bind _blackboard (`AIController.Blackboard` (`AIBlueprintHelperLibrary.GetAIController` _returnvalue)))
  (bind _asdrflying_enemy (cast `DRFlyingEnemy` (`self.GetAvatarActorFromActorInfo`)))
  (`DREnemy.OnAttackExecuted` _asdrflying_enemy)
  (`AbilityTask_PlayMontageAndWait.CreatePlayMontageAndWaitProxy` "None" _montage
    (:`then`
      (`AbilityTask_WaitGameplayEvent.WaitGameplayEvent` _montagetag null true
        (:`EventReceived`
          (bind _returnvalue_2 (message `EnemyInterface.GetCombatTarget` _returnvalue))
          (`self.SpawnProjectile` (`Actor.K2_GetActorLocation` _returnvalue_2) _sockettag (`self.ShouldOverridePitch`) (`self.PitchOverride`))
          (`BlackboardComponent.SetValueAsInt` _blackboard (`self.BasicAttackCount`) (+ (`BlackboardComponent.GetValueAsInt` _blackboard (`self.BasicAttackCount`)) 1)))))
    (:`OnCompleted`
      (`self.K2_EndAbility` :!label _label))
    (:`OnInterrupted`
      (goto _label))
    (:`OnCancelled`
      (goto _label))))