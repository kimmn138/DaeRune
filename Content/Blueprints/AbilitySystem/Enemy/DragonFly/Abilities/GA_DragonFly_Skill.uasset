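; Skill ability for the DragonFly flying enemy that fires a projectile at its combat target during a montage.
; On activation it notifies the enemy of the attack, plays the tagged montage and waits for that montage's gameplay event.
; The event spawns a projectile from the tagged socket toward the target's location, with optional pitch override.
; When the montage ends or is interrupted, it resets the Blackboard basic attack count, starts skill lockdown and ends the ability.
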(event `self.K2_ActivateAbility`
  (bind _returnvalue (`self.GetAvatarActorFromActorInfo`))
  (bind (_montage _montagetag _sockettag) (break `TaggedMontage` (`self.TaggedMontage`)))
  (bind _asdrflying_enemy (cast `DRFlyingEnemy` (`self.GetAvatarActorFromActorInfo`)))
  (`DREnemy.OnAttackExecuted` _asdrflying_enemy)
  (`AbilityTask_PlayMontageAndWait.CreatePlayMontageAndWaitProxy` "None" _montage
    (:`then`
      (`AbilityTask_WaitGameplayEvent.WaitGameplayEvent` _montagetag null
        (:`EventReceived`
          (bind _returnvalue_2 (message `EnemyInterface.GetCombatTarget` _returnvalue))
          (`self.SpawnProjectile` (`Actor.K2_GetActorLocation` _returnvalue_2) _sockettag (`self.ShouldOverridePitch`) (`self.PitchOverride`)))))
    (:`OnCompleted`
      (`BlackboardComponent.SetValueAsInt` (`AIController.Blackboard` (`AIBlueprintHelperLibrary.GetAIController` _returnvalue)) (`self.BasicAttackCount`) 0 :!label _label)
      (`DRFlyingEnemy.StartSkillLockdown` _asdrflying_enemy)
      (`self.K2_EndAbility`))
    (:`OnInterrupted`
      (goto _label))
    (:`OnCancelled`
      (goto _label))))