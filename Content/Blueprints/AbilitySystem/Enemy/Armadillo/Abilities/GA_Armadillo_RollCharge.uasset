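; Armadillo enemy gameplay ability that morphs into ball form and roll-charges at the saved location of the blackboard's target character.
; Chained form-change montages across two meshes lead into the charge, which reports back through impact and reached-target delegates.
; Impacts damage characters and cleanser sites (scaled), stun non-friends, and self-stun the armadillo when no player or enemy is hit.
; Both outcomes revert form, commit cooldown, flag the blackboard and end the ability.
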(event `self.K2_ActivateAbility`
  (bind _drarmadillo_enemy (`self.DRArmadillo Enemy`))
  (bind _drarmadillo_enemy_2 (`self.DRArmadillo Enemy`))
  (bind _drarmadillo_enemy_3 (`self.DRArmadillo Enemy`))
  (bind _asdrarmadillo_enemy (cast `DRArmadilloEnemy` (`self.GetAvatarActorFromActorInfo`)))
  (bind _output_get (set `self.DRArmadillo Enemy` _asdrarmadillo_enemy))
  (bind _asdraicontroller (cast `DRAIController` (`AIBlueprintHelperLibrary.GetAIController` _output_get)))
  (bind _output_get_2 (set `self.DRAIController` _asdraicontroller))
  (bind _blackboard (`AIController.Blackboard` _output_get_2))
  (`BlackboardComponent.SetValueAsBool` _blackboard (`self.bIsRollSkillEnd`) false)
  (bind _asdrcharacter (cast `DRCharacter` (`BlackboardComponent.GetValueAsObject` _blackboard (`self.TargetToRoll`))))
  (set `self.SavedTargetLocation` (`Actor.K2_GetActorLocation` _asdrcharacter))
  (add `DRArmadilloEnemy.OnRollImpact` _drarmadillo_enemy (delegate `HandleRollImpact`))
  (add `DRArmadilloEnemy.OnRollReachedTarget` _drarmadillo_enemy (delegate `HandleRollReachedTarget`))
  (`/Engine/EditorBlueprintResources/StandardMacros.IsValid` _drarmadillo_enemy_2
    (:`Is Valid`
      (`DRArmadilloEnemy.StartFormChange` _drarmadillo_enemy_2 true)
      (`|PlayMontage` (`Character.Mesh` _drarmadillo_enemy_2) "/Game/DaeRuneAssets/Characters/Enemy/Armadilo/BasicForm/AM_Armadillo_FormChangeDtoB.AM_Armadillo_FormChangeDtoB" 2.0
        (:`OnCompleted`
          (`DRArmadilloEnemy.FinishFormChange` _drarmadillo_enemy_3)
          (`|PlayMontage` (`DRArmadilloEnemy.BallFormMesh` _drarmadillo_enemy_3) "/Game/DaeRuneAssets/Characters/Enemy/Armadilo/RollForm/AM_Armadillo_Ball_FormChangeDtoB.AM_Armadillo_Ball_FormChangeDtoB" 2.0
            (:`OnCompleted`
              _)
            (:`OnInterrupted`
              _))
          (`DRArmadilloEnemy.StartRollCharge` (`self.DRArmadillo Enemy`) (`self.SavedTargetLocation`))
          (`DREnemy.OnAttackExecuted` (`self.DRArmadillo Enemy`)))))))

(event `HandleRollImpact`
  (params (ImpactResult :type "RollImpactResult Structure (by ref)"))
  (bind _returnvalue (`self.GetAbilitySystemComponentFromActorInfo`))
  (bind _returnvalue_2 (`self.GetAvatarActorFromActorInfo`))
  (bind _drarmadillo_enemy (`self.DRArmadillo Enemy`))
  (bind _drarmadillo_enemy_2 (`self.DRArmadillo Enemy`))
  (for _array_element ImpactResult_HitActors
    (bind _asdrcharacter_base (cast `DRCharacterBase` _array_element)
      (:`then`
        (`DRAbilitySystemLibrary.ApplyDamageEffect` (`self.MakeDamageEffectParamsFromClassDefaults` _asdrcharacter_base))
        (if (`DRAbilitySystemLibrary.IsNotFriend` _asdrcharacter_base _returnvalue_2)
          (bind _returnvalue_3 (`AbilitySystemBlueprintLibrary.GetAbilitySystemComponent` _asdrcharacter_base))
          (`AbilitySystemComponent.BP_ApplyGameplayEffectSpecToTarget` (`AbilitySystemBlueprintLibrary.GetAbilitySystemComponent` _returnvalue_2) (`AbilitySystemComponent.MakeOutgoingSpec` :`self` _returnvalue_3 :`GameplayEffectClass` "/Game/Blueprints/AbilitySystem/Enemy/Armadillo/Effects/GE_AramadilloRollStun_Player.GE_AramadilloRollStun_Player_C" :`Level` 1.0) _returnvalue_3)))
      (:`CastFailed`
        (bind _asdrcleanser_site (cast `DRCleanserSite` _array_element))
        (bind (_returnvalue_worldcontextobject _returnvalue_damagegameplayeffectclass _returnvalue_sourceabilitysystemcomponent _returnvalue_targetabilitysystemcomponent _returnvalue_basedamage _returnvalue_abilitylevel _returnvalue_damagetype _returnvalue_debuffchance _returnvalue_debuffdamage _returnvalue_debuffduration _returnvalue_deathimpulsemagnitude _returnvalue_deathimpulse _returnvalue_knockbackforcemagnitude _returnvalue_knockbackchance _returnvalue_knockbackforce _returnvalue_sourceabilitytags) (break `DamageEffectParams` (`self.MakeDamageEffectParamsFromClassDefaults` _asdrcleanser_site)))
        (`DRAbilitySystemLibrary.ApplyDamageEffect` (make `DamageEffectParams` _returnvalue_worldcontextobject _returnvalue_damagegameplayeffectclass _returnvalue_sourceabilitysystemcomponent _returnvalue_targetabilitysystemcomponent (* _returnvalue_basedamage (`self.CleanserDamageMultiplier`)) _returnvalue_abilitylevel _returnvalue_damagetype _returnvalue_debuffchance _returnvalue_debuffdamage _returnvalue_debuffduration _returnvalue_deathimpulsemagnitude _returnvalue_deathimpulse _returnvalue_knockbackforcemagnitude _returnvalue_knockbackchance _returnvalue_knockbackforce _returnvalue_sourceabilitytags)))))
  (`/Engine/EditorBlueprintResources/StandardMacros.IsValid` (`self.DRArmadillo Enemy`)
    (:`Is Valid`
      (if (not ImpactResult_bHitPlayerOrEnemy)
        (`AbilitySystemComponent.BP_ApplyGameplayEffectSpecToSelf` _returnvalue (`AbilitySystemComponent.MakeOutgoingSpec` :`self` _returnvalue :`GameplayEffectClass` "/Game/Blueprints/AbilitySystem/Enemy/Armadillo/Effects/GE_ArmadilloRollStun_Self.GE_ArmadilloRollStun_Self_C" :`Level` 1.0)))
      (`DRArmadilloEnemy.StartFormChange` _drarmadillo_enemy false)
      (`|PlayMontage` (`DRArmadilloEnemy.BallFormMesh` _drarmadillo_enemy) "/Game/DaeRuneAssets/Characters/Enemy/Armadilo/RollForm/AM_Armadillo_Ball_FormChangeBtoD.AM_Armadillo_Ball_FormChangeBtoD" 2.0
        (:`OnCompleted`
          (`DRArmadilloEnemy.FinishFormChange` _drarmadillo_enemy_2)
          (`|PlayMontage` (`Character.Mesh` _drarmadillo_enemy_2) "/Game/DaeRuneAssets/Characters/Enemy/Armadilo/BasicForm/AM_Armadillo_FormChangeBtoD.AM_Armadillo_FormChangeBtoD" 2.0
            (:`OnCompleted`
              (`self.K2_CommitAbilityCooldown` false)
              (`BlackboardComponent.SetValueAsBool` (`AIController.Blackboard` (`self.DRAIController`)) (`self.bIsRollSkillEnd`) true)
              (`self.K2_EndAbility`))))))))

(event `HandleRollReachedTarget`
  (bind _drarmadillo_enemy (`self.DRArmadillo Enemy`))
  (bind _drarmadillo_enemy_2 (`self.DRArmadillo Enemy`))
  (`/Engine/EditorBlueprintResources/StandardMacros.IsValid` _drarmadillo_enemy_2
    (:`Is Valid`
      (`DRArmadilloEnemy.StartFormChange` _drarmadillo_enemy_2 false)
      (`|PlayMontage` (`DRArmadilloEnemy.BallFormMesh` _drarmadillo_enemy_2) "/Game/DaeRuneAssets/Characters/Enemy/Armadilo/RollForm/AM_Armadillo_Ball_FormChangeBtoD.AM_Armadillo_Ball_FormChangeBtoD" 2.0
        (:`OnCompleted`
          (`DRArmadilloEnemy.FinishFormChange` _drarmadillo_enemy)
          (`|PlayMontage` (`Character.Mesh` _drarmadillo_enemy) "/Game/DaeRuneAssets/Characters/Enemy/Armadilo/BasicForm/AM_Armadillo_FormChangeBtoD.AM_Armadillo_FormChangeBtoD" 2.0
            (:`OnCompleted`
              (`self.K2_CommitAbilityCooldown` false)
              (`BlackboardComponent.SetValueAsBool` (`AIController.Blackboard` (`self.DRAIController`)) (`self.bIsRollSkillEnd`) true)
              (`self.K2_EndAbility`))))))))