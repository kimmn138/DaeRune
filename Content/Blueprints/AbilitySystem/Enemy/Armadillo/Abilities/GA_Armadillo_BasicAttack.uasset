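; Gameplay ability for the Armadillo enemy's basic melee attack, notifying the avatar DREnemy that an attack has executed.
; It plays a tagged montage and waits for that montage's gameplay event.
; On the event, it gathers live actors within a small sphere at the tagged combat socket, damages non-friends using class-default effect params, and ends.
; Montage interruption or cancellation also ends it.
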(event `self.K2_ActivateAbility`
  (bind _returnvalue (`self.GetAvatarActorFromActorInfo`))
  (bind (_montage _montagetag _sockettag) (break `TaggedMontage` (`self.TaggedMontage`)))
  (bind _asdrenemy (cast `DREnemy` (`self.GetAvatarActorFromActorInfo`)))
  (`DREnemy.OnAttackExecuted` _asdrenemy)
  (`AbilityTask_PlayMontageAndWait.CreatePlayMontageAndWaitProxy` "None" _montage 1.0 "None" false
    (:`then`
      (`AbilityTask_WaitGameplayEvent.WaitGameplayEvent` _montagetag null
        (:`EventReceived`
          (bind _returnvalue_2 (message `CombatInterface.GetCombatSocketLocation` _returnvalue _sockettag))
          (set `self.CombatSocketLocation` _returnvalue_2)
          (bind _outoverlappingactors (`DRAbilitySystemLibrary.GetLiveObjectsWithinRadius` _returnvalue (`|MakeArray` _returnvalue) 30.0 (`self.CombatSocketLocation`)))
          (for _array_element _outoverlappingactors
            (if (`DRAbilitySystemLibrary.IsNotFriend` (`self.GetAvatarActorFromActorInfo`) _array_element)
              (`DRAbilitySystemLibrary.ApplyDamageEffect` (`self.MakeDamageEffectParamsFromClassDefaults` _array_element))))
          (`self.K2_EndAbility`))))
    (:`OnInterrupted`
      (`self.K2_EndAbility` :!label _label))
    (:`OnCancelled`
      (goto _label))))