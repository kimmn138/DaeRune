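; GA_ClawSwipe is the Garden Robot's Skill 1 melee ability, damaging valid targets and trying to heal allies with the robot's own health.
; A tagged montage plays at windup rate, alongside a first-person shovel-attack montage when locally controlled.
; The montage's gameplay event restores play rate and triggers an upgrade-scaled radius query at the combat socket.
; The ability ends when the tagged montage completes, blends out or is interrupted.
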(event `self.K2_ActivateAbility`
  (bind _returnvalue (`self.GetWindupPlayRate`))
  (bind _returnvalue_2 (`self.GetAvatarActorFromActorInfo`))
  (bind (_taggedmontage_montage _taggedmontage_montagetag _taggedmontage_sockettag) (break `TaggedMontage` (`self.TaggedMontage`)))
  (bind _asbp_garden_robot (cast `/Game/Blueprints/Character/PlayerCharacter/GardenRobot/BP_GardenRobot` (`self.GetAvatarActorFromActorInfo`)))
  (`self.IsLocallyControlled`
    (:`True`
      (`|PlayMontage` (`DRCharacter.FirstPersonMesh` _asbp_garden_robot) "/Game/DaeRuneAssets/Characters/GardenRobot_v3/FP/AM_Gardener_ShovelAttack1.AM_Gardener_ShovelAttack1" _returnvalue
        (:`then`
          _)))
    (:`False`
      _))
  (`AbilityTask_PlayMontageAndWait.CreatePlayMontageAndWaitProxy` "None" _taggedmontage_montage _returnvalue "None" false
    (:`then`
      (`AbilityTask_WaitGameplayEvent.WaitGameplayEvent` _taggedmontage_montagetag null true
        (:`EventReceived`
          (`self.RestoreMontagePlayRate`)
          (bind _returnvalue_3 (message `CombatInterface.GetCombatSocketLocation` _returnvalue_2 _taggedmontage_sockettag))
          (bind _output_get (set `self.CombatSocketLocation` _returnvalue_3))
          (bind _outoverlappingactors (`DRAbilitySystemLibrary.GetLiveObjectsWithinRadius` _returnvalue_2 (`|MakeArray` _returnvalue_2) (`self.GetUpgradedAttackRadius`) _output_get))
          (for _array_element _outoverlappingactors
            (if (`DRAbilitySystemLibrary.IsValidDamageTarget` (`self.GetAvatarActorFromActorInfo`) _array_element)
              (`DRAbilitySystemLibrary.ApplyDamageEffect` (`self.MakeDamageEffectParamsFromClassDefaults` _array_element))
              (else
                (`self.TryHealAllyWithOwnHealth` _array_element)))))))
    (:`OnCompleted`
      (`self.K2_EndAbility` :!label _label))
    (:`OnBlendOut`
      (goto _label))
    (:`OnInterrupted`
      (goto _label))
    (:`OnCancelled`
      (goto _label))))