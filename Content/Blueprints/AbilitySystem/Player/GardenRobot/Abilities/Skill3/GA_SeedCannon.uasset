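; Gameplay ability for the Garden Robot's third skill, Seed Cannon, which fires a seed projectile.
; Activation commits only the cost, plays a first-person montage for local players, then plays the tagged montage for all paths, both scaled by attack speed.
; The montage's gameplay event makes the authority spawn the projectile from a first-person mesh socket along the camera's forward vector.
; The ability ends when the montage completes, blends out or is interrupted or cancelled.
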(event `self.K2_ActivateAbility`
  (bind _returnvalue (`self.GetAttackSpeedPlayRate`))
  (bind (_taggedmontage_montage _taggedmontage_montagetag) (break `TaggedMontage` (`self.TaggedMontage`)))
  (bind _asbp_garden_robot (cast `/Game/Blueprints/Character/PlayerCharacter/GardenRobot/BP_GardenRobot` (`self.GetAvatarActorFromActorInfo`)))
  (`self.K2_CommitAbilityCost` false)
  (`self.IsLocallyControlled`
    (:`True`
      (bind _firstpersonmesh (`DRCharacter.FirstPersonMesh` _asbp_garden_robot))
      (`|PlayMontage` _firstpersonmesh "/Game/DaeRuneAssets/Characters/GardenRobot_v3/FP/AM_Gardener_SeedBomb.AM_Gardener_SeedBomb" _returnvalue
        (:`then`
          _)))
    (:`False`
      _))
  (`AbilityTask_PlayMontageAndWait.CreatePlayMontageAndWaitProxy` "None" _taggedmontage_montage _returnvalue "None" false
    (:`then`
      (`AbilityTask_WaitGameplayEvent.WaitGameplayEvent` _taggedmontage_montagetag null true
        (:`EventReceived`
          (bind _ascharacter (cast `Character` (`self.GetAvatarActorFromActorInfo`)))
          (bind _asplayer_controller (cast `PlayerController` (`Pawn.GetController` _ascharacter)))
          (`self.K2_HasAuthority`
            (:`True`
              (`self.SpawnSeedProjectile` (`KismetMathLibrary.GetForwardVector` (`PlayerCameraManager.GetCameraRotation` (`PlayerController.PlayerCameraManager` _asplayer_controller))) (`SceneComponent.GetSocketLocation` _firstpersonmesh "TestTail")))))))
    (:`OnCompleted`
      (`self.K2_EndAbility` :!label _label))
    (:`OnBlendOut`
      (goto _label))
    (:`OnInterrupted`
      (goto _label))
    (:`OnCancelled`
      (goto _label))))