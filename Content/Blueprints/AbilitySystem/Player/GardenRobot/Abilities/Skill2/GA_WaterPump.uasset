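; Garden Robot's second skill, a held Water Pump ability that damages hostile targets and grants water to allies.
; Activation plays start montages, with a first-person one for the local player, then a montage gameplay event starts the pump loop and a looping timer that commits cost.
; Each damage tick checks friendliness and applies damage or water on authority only.
; Releasing input stops the loop and timer, then ends the ability after a brief delay.
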(event `self.K2_ActivateAbility`
  (bind (_taggedmontage_montage _taggedmontage_montagetag) (break `TaggedMontage` (`self.TaggedMontage`)))
  (bind _asbp_garden_robot (cast `/Game/Blueprints/Character/PlayerCharacter/GardenRobot/BP_GardenRobot` (`self.GetAvatarActorFromActorInfo`)))
  (`|ExecutionSequence`
    (:`then_0`
      (`self.IsLocallyControlled`
        (:`True`
          (`|PlayMontage` (`DRCharacter.FirstPersonMesh` _asbp_garden_robot) "/Game/DaeRuneAssets/Characters/GardenRobot_v3/FP/AM_Gardener_FP_WaterBlast_Start.AM_Gardener_FP_WaterBlast_Start"
            (:`then`
              _)))
        (:`False`
          _))
      (`AbilityTask_PlayMontageAndWait.CreatePlayMontageAndWaitProxy` "None" _taggedmontage_montage
        (:`then`
          (`AbilityTask_WaitGameplayEvent.WaitGameplayEvent` _taggedmontage_montagetag null true
            (:`EventReceived`
              (message `CombatInterface.SetInWaterLoop` (`self.GetAvatarActorFromActorInfo`) true)
              (`self.StartWaterPumpLoop`)
              (bind _returnvalue (`KismetSystemLibrary.K2_SetTimerDelegate` (delegate `Cost`) (`self.DamageDeltaTime`) true))
              (set `self.DamageAndCostTimer` _returnvalue))))))
    (:`then_1`
      (`AbilityTask_WaitInputRelease.WaitInputRelease` true
        (:`OnRelease`
          (message `CombatInterface.SetInWaterLoop` (`self.GetAvatarActorFromActorInfo`) false)
          (`self.StopWaterPumpLoop`)
          (`KismetSystemLibrary.K2_ClearAndInvalidateTimerHandle` (`self.DamageAndCostTimer`))
          (`KismetSystemLibrary.Delay` 0.1)
          (`self.K2_EndAbility`))))))

(event `Cost`
  (`self.K2_CommitAbilityCost` false))

(event `self.OnDamageTickReached`
  (params (Target :type "Actor Object Reference"))
  (bind _targetactor (`self.TargetActor`))
  (set `self.TargetActor` Target)
  (if (`DRAbilitySystemLibrary.IsNotFriend` (`self.GetAvatarActorFromActorInfo`) _targetactor)
    (`self.K2_HasAuthority`
      (:`True`
        (`DRAbilitySystemLibrary.ApplyDamageEffect` (`self.MakeDamageEffectParamsFromClassDefaults` _targetactor))))
    (else
      (`self.K2_HasAuthority`
        (:`True`
          (bind _asdrcharacter (cast `DRCharacter` (`self.TargetActor`)))
          (`self.GrantWaterToAlly` _asdrcharacter))))))

(fn `EnforceImplementsCombatInterface`
  (if (not (`KismetSystemLibrary.DoesImplementInterface` (`self.GetAvatarActorFromActorInfo`) "/Script/DaeRune.CombatInterface"))
    (`self.K2_EndAbility`)))

(fn `SpawnWaterPump`
  (params (TargetLocation :type "Vector Structure") (WeaponSocketLocation :type "Vector Structure")))