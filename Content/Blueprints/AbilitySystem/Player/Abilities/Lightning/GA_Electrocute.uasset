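; Player lightning ability that plays the Electrocute montage and holds the avatar in a shock loop until input is released.
; On activation it stores camera target data, turns the avatar toward the hit location and fires the ShockBurst gameplay cue.
; A montage gameplay event starts the loop through CombatInterface and disables movement; releasing input clears the loop, restores walking and ends the ability.
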(event `self.K2_ActivateAbility`
  (`self.EnforceImplementsCombatInterface`)
  ; Store Camera Data Variables
  (bind (_asynctaskproxy _datahandle) (`TargetDataFromCamera.CreateTargetDataFromCamera` 0.0)
    (:`ValidData`
      (`self.StoreCameraDataInfo` (`AbilitySystemBlueprintLibrary.GetHitResultFromTargetData` _datahandle))
      (`self.StoreOwnerVariables`)
      (`|ExecutionSequence`
        (:`then_0`
          (`self.UpdateFacingTarget`)
          (`self.K2_ExecuteGameplayCue` (struct :`TagName` "GameplayCue.ShockBurst"))
          (`AbilityTask_PlayMontageAndWait.CreatePlayMontageAndWaitProxy` "None" (`self.Montage_Electrocute`) 1.0 "None" false
            (:`then`
              (`AbilityTask_WaitGameplayEvent.WaitGameplayEvent` (struct :`TagName` "Event.Montage.Electrocute") null true
                (:`EventReceived`
                  (`self.InShockLoop`))))))
        (:`then_1`
          (`AbilityTask_WaitInputRelease.WaitInputRelease` false
            (:`OnRelease`
              (`self.PrepareToEndAbility`)
              (`self.K2_EndAbility`))))))))

(fn `EnforceImplementsCombatInterface`
  (if (not (`KismetSystemLibrary.DoesImplementInterface` (`self.GetAvatarActorFromActorInfo`) "/Script/DaeRune.CombatInterface"))
    (`self.K2_EndAbility`)))

(fn `InShockLoop`
  (message `CombatInterface.SetInShockLoop` (`self.GetAvatarActorFromActorInfo`) true)
  (`CharacterMovementComponent.DisableMovement` (`Character.CharacterMovement` (`self.OwnerCharacter`))))

(fn `PrepareToEndAbility`
  (message `CombatInterface.SetInShockLoop` (`self.GetAvatarActorFromActorInfo`) false)
  (`CharacterMovementComponent.SetMovementMode` (`Character.CharacterMovement` (`self.OwnerCharacter`)) "MOVE_Walking" 0))

(fn `UpdateFacingTarget`
  (message `CombatInterface.UpdateFacingTarget` (`self.GetAvatarActorFromActorInfo`) (`self.CameraHitLocation`)))