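; Gameplay ability for the Vending Machine character's basic attack, which auto-fires while input is held.
; Activation starts auto fire from the parent class and waits for input release to stop firing and end the ability.
; Capsule shots play an attack montage on the body mesh, plus a first-person one when locally controlled.
; Normal shot and jackpot stack events are empty stubs.
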(event `self.K2_ActivateAbility`
  (`|ExecutionSequence`
    (:`then_0`
      (`self.StartAutoFire`))
    (:`then_1`
      (`AbilityTask_WaitInputRelease.WaitInputRelease` false
        (:`OnRelease`
          (`self.StopAutoFire`)
          (`self.K2_EndAbility`))))))

(event `self.OnNormalShotFired`)

(event `self.OnCapsuleShotFired`
  (params (CapsuleTier :type Integer))
  (bind _asbp_drvending_machine (cast `/Game/Blueprints/Character/PlayerCharacter/VendingMachine/BP_VendingMachine` (`self.GetAvatarActorFromActorInfo`)))
  (`self.IsLocallyControlled`
    (:`True`
      (`|PlayMontage` (`DRCharacter.FirstPersonMesh` _asbp_drvending_machine) "/Game/DaeRuneAssets/Characters/VendingMachine/FP/AM_VM_FP_CapsuleAttack.AM_VM_FP_CapsuleAttack" :!label _label
        (:`then`
          (`|PlayMontage` (`Character.Mesh` _asbp_drvending_machine) "/Game/DaeRuneAssets/Characters/VendingMachine/TP/AM_VM_CapsuleAttack.AM_VM_CapsuleAttack" :!label _label_2
            (:`then`
              (switch `int` CapsuleTier
                (:`0`
                  (goto _label))))))))
    (:`False`
      (goto _label_2))))

(event `self.OnJackpotStacksChanged`
  (params (NewStacks :type Integer) (MaxStacks :type Integer)))