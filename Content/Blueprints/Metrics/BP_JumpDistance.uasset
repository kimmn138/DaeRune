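; BP_JumpDistance is a metrics ruler actor that shows the distance between its Start and End components, such as for measuring jumps.
; RebuildRuler draws a two-point spline mesh between them and places a label above the midpoint showing the raw world-unit distance plus CustomLabel.
; It runs on construction and every Tick, which also turns the label to face the player camera.
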(event `self.ReceiveTick`
  (params (DeltaSeconds :type "Float (single-precision)"))
  (bind _label (`self.Label`))
  (`self.RebuildRuler` :!label _label)
  (`SceneComponent.K2_SetWorldRotation` _label (`KismetMathLibrary.FindLookAtRotation` (`SceneComponent.K2_GetComponentLocation` _label) (`PlayerCameraManager.GetCameraLocation` (`GameplayStatics.GetPlayerCameraManager` 0))) false false))

(event `self.Start.OnReleased`
  (params (TouchedComponent :type "PrimitiveComponent Object Reference") (ButtonReleased :type "Key Structure"))
  (goto _label))

(fn `RebuildRuler`
  (bind _start (`self.Start`))
  (bind _end (`self.End`))
  (bind _splinemesh (`self.SplineMesh`))
  (bind _spline (`self.Spline`))
  (bind _label (`self.Label`))
  (bind _returnvalue (`SceneComponent.K2_GetComponentLocation` _start))
  (bind _returnvalue_2 (`SceneComponent.K2_GetComponentLocation` _end))
  (bind _output_get (set `self.StartLoc` (`SceneComponent.RelativeLocation` _start)))
  (bind _output_get_2 (set `self.EndLoc` (`SceneComponent.RelativeLocation` _end)))
  (`SplineComponent.ClearSplinePoints` _spline true)
  (`SplineComponent.AddSplinePoint` _spline _output_get "Local" true)
  (`SplineComponent.AddSplinePoint` _spline _output_get_2 "Local" true)
  (`SplineComponent.SetClosedLoop` _spline false true)
  (`SplineMeshComponent.SetStartAndEnd` _splinemesh (`SplineComponent.GetLocationAtSplinePoint` _spline 0 "Local") (`SplineComponent.GetTangentAtSplinePoint` _spline 0 "Local") (`SplineComponent.GetLocationAtSplinePoint` _spline 1 "Local") (`SplineComponent.GetTangentAtSplinePoint` _spline 1 "Local") true)
  (`SplineMeshComponent.SetStartScale` _splinemesh (0.1 0.1) true)
  (`SplineMeshComponent.SetEndScale` _splinemesh (0.1 0.1) true)
  (`SceneComponent.K2_SetWorldLocation` _label (+ (* (+ _returnvalue_2 _returnvalue) 0.5) (10.0 10.0 30.0)) false false)
  (`TextRenderComponent.K2_SetText` _label (`|FormatText` "{D} \n{label}" (`KismetTextLibrary.Conv_DoubleToText` (`KismetMathLibrary.VSize` (- _returnvalue_2 _returnvalue)) "HalfToEven") (`self.CustomLabel`))))

(fn `UserConstructionScript`
  (`self.RebuildRuler`))