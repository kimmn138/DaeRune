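; Player controller that shows a cleanser part pickup notice and provides debug hotkeys.
; On part pickup it reaches the stage overlay widget through the stage HUD, makes the notice visible, then collapses it with a short function-name timer.
; The 0 key calls the cheat to skip to the next phase, and 9 toggles first-person mesh and HUD visibility.
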(event `Key|Zero`
  (params (Key :type "Key Structure"))
  (:`Pressed`
    (`self.CheatSkipToNextPhase`)))

(event `self.OnPartPickedUp`
  (bind _asbp_drstage_hud (cast `/Game/Blueprints/UI/HUD/BP_DRStageHUD` (`self.GetHUD`)))
  (bind _aswbp_stage_overlay (cast `/Game/Blueprints/UI/Overlay/WBP_StageOverlay` (`DRHUD.GetOverlayWidget` _asbp_drstage_hud)))
  (`Widget.SetVisibility` (`/Game/Blueprints/UI/Overlay/WBP_StageOverlay.WBP_PickupCleanserPart` _aswbp_stage_overlay) "Visible")
  (`KismetSystemLibrary.K2_SetTimer` null "HidePartUI" 2.0))

(event `Key|Nine`
  (params (Key :type "Key Structure"))
  (:`Pressed`
    (`self.ToggleFirstPersonMeshAndHUDVisibility`)))

(fn `HidePartUI`
  (bind _asbp_drstage_hud (cast `/Game/Blueprints/UI/HUD/BP_DRStageHUD` (`self.GetHUD`)))
  (bind _aswbp_stage_overlay (cast `/Game/Blueprints/UI/Overlay/WBP_StageOverlay` (`DRHUD.GetOverlayWidget` _asbp_drstage_hud)))
  (`Widget.SetVisibility` (`/Game/Blueprints/UI/Overlay/WBP_StageOverlay.WBP_PickupCleanserPart` _aswbp_stage_overlay) "Collapsed"))

(fn `UserConstructionScript`)