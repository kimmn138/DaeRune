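; BP_S2SwitchPuzzle is the visual layer of a Stage 2 switch puzzle, showing bulb states and cleared rounds.
; BeginPlay creates dynamic material instances for nine bulb meshes and three round-light meshes.
; OnBulbsChanged decodes a bitmask to light bulbs purple or black them out through EmissiveFactor.
; OnRoundsClearedChanged turns round lights green up to the cleared count but never resets them; the puzzle logic itself is outside this graph.
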(event `self.ReceiveBeginPlay`
  (bind _output_get (set `self.Bulbs` (`|MakeArray` (`self.StaticMesh1`) (`self.StaticMesh2`) (`self.StaticMesh3`) (`self.StaticMesh4`) (`self.StaticMesh5`) (`self.StaticMesh6`) (`self.StaticMesh7`) (`self.StaticMesh8`) (`self.StaticMesh9`))))
  (for _array_element _output_get
    (bind _returnvalue (`PrimitiveComponent.CreateDynamicMaterialInstance` _array_element 0 "/Game/DaeRuneAssets/Map/Stage2_v1/Puzzle/stage2_purple_M.stage2_purple_M" "None"))
    (`KismetArrayLibrary.Array_Add` (`self.BulbsMIDs`) _returnvalue))
  (bind _output_get_2 (set `self.RountLights` (`|MakeArray` (`self.StaticMesh11`) (`self.StaticMesh12`) (`self.StaticMesh13`))))
  (for _array_element_2 _output_get_2
    (bind _returnvalue_2 (`PrimitiveComponent.CreateDynamicMaterialInstance` _array_element_2 0 "/Game/DaeRuneAssets/Map/Stage2_v1/Puzzle/Material_001.Material_001" "None"))
    (`KismetArrayLibrary.Array_Add` (`self.RoundLightsMIDs`) _returnvalue_2)))

(event `self.OnBulbsChanged`
  (params (NewBulbBits :type Integer))
  (`KismetSystemLibrary.PrintString` (`KismetStringLibrary.Conv_IntToString` (`KismetArrayLibrary.Array_Length` (`self.BulbsMIDs`))))
  (for _index (range 9)
    (if (`self.IsBitSet` NewBulbBits _index)
      (`MaterialInstanceDynamic.SetVectorParameterValue` (`|GetArrayItem` (`self.BulbsMIDs`) _index) "EmissiveFactor" (make `LinearColor` 3.07357 0.17703 3.84263 1.0))
      (else
        (`MaterialInstanceDynamic.SetVectorParameterValue` (`|GetArrayItem` (`self.BulbsMIDs`) _index) "EmissiveFactor" (make `LinearColor` 0.0 0.0 0.0 1.0))))))

(event `self.OnRoundsClearedChanged`
  (params (NewRoundsCleared :type Integer))
  (`KismetSystemLibrary.PrintString` (`KismetStringLibrary.Conv_IntToString` (`KismetArrayLibrary.Array_Length` (`self.RoundLightsMIDs`))))
  (for _index (range 3)
    (if (< _index NewRoundsCleared)
      (`MaterialInstanceDynamic.SetVectorParameterValue` (`|GetArrayItem` (`self.RoundLightsMIDs`) _index) "EmissiveFactor" (make `LinearColor` 0.91182 8.0 0.83461 1.0)))))

(fn `UserConstructionScript`)