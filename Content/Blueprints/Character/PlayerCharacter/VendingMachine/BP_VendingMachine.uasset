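; BP_VendingMachine is a player character Blueprint that shows the player's name overhead and animates a death camera.
; Two seconds after BeginPlay, it casts its overhead widget child actor and player state, then passes the player name to the widget.
; PlayDeathCameraAnimation runs a timeline that lerps the follow camera from the actor's location to high above it, sweeping for collision, while pitching it straight down.
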(event `self.ReceiveBeginPlay`
  (`KismetSystemLibrary.Delay` 2.0)
  (bind _asbp_overhead_widget (cast `/Game/Blueprints/UI/FloatingText/BP_OverheadWidget` (`ChildActorComponent.ChildActor` (`self.OverheadWidget1`))))
  (bind _asbp_drplayer_state (cast `/Game/Blueprints/Player/BP_DRPlayerState` (`self.PlayerState`)))
  (`/Game/Blueprints/UI/FloatingText/BP_OverheadWidget.ShowOverheadWidget` _asbp_overhead_widget (`PlayerState.GetPlayerName` _asbp_drplayer_state)))

(event `self.PlayDeathCameraAnimation`
  (bind (_returnvalue_x _returnvalue_y _returnvalue_z) (`KismetMathLibrary.BreakVector` (`self.K2_GetActorLocation`)))
  (bind _returnvalue (`self.GetFollowCamera`))
  (bind (_direction _cameratransition) (`Timeline|DeathCameraTimeline`)
    (:`Update`
      (`SceneComponent.K2_SetWorldLocation` _returnvalue (`KismetMathLibrary.MakeVector` _returnvalue_x _returnvalue_y (+ _returnvalue_z (`KismetMathLibrary.Lerp` 0.0 400.0 _cameratransition))) true false)
      (`SceneComponent.K2_SetWorldRotation` _returnvalue (`KismetMathLibrary.MakeRotator` 0.0 (`KismetMathLibrary.Lerp` 0.0 -90.0 _cameratransition)) false false))))

(fn `UserConstructionScript`)